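; First aid kit pickup that heals the player's FirstPersonCharacter when it overlaps the kit.
; If health is below maximum, it adds a fixed amount capped at MaxHealth; at full health the kit stays in place.
; On use it sets the character's first-aid flags, turns off rendering of its healing Niagara effect, and destroys itself after a short delay.
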(event Collision|EventActorBeginOverlap
  (params (OtherActor :type Actor%20Object%20Reference))
  (bind _returnvalue (Game|GetPlayerCharacter 0))
  ;[1 1 1] Add Health points
  (if (== OtherActor _returnvalue)
    (bind _asfirst_person_character (Utilities|Casting|CastToFirstPersonCharacter _returnvalue))
    (if (not (== (Variables|/Game/MyProject/Blueprints/Player/FirstPersonCharacter.FirstPersonCharacter_C|GetMaxHealth _asfirst_person_character) (Variables|/Game/MyProject/Blueprints/Player/FirstPersonCharacter.FirstPersonCharacter_C|GetCurrentHealth _asfirst_person_character)))
      (if (<= (Variables|/Game/MyProject/Blueprints/Player/FirstPersonCharacter.FirstPersonCharacter_C|GetMaxHealth _asfirst_person_character) (+ (Variables|/Game/MyProject/Blueprints/Player/FirstPersonCharacter.FirstPersonCharacter_C|GetCurrentHealth _asfirst_person_character) 5e+01))
        (Variables|/Game/MyProject/Blueprints/Player/FirstPersonCharacter.FirstPersonCharacter_C|SetCurrentHealth _asfirst_person_character (Variables|/Game/MyProject/Blueprints/Player/FirstPersonCharacter.FirstPersonCharacter_C|GetMaxHealth _asfirst_person_character))
        (else
          (Variables|/Game/MyProject/Blueprints/Player/FirstPersonCharacter.FirstPersonCharacter_C|SetCurrentHealth _asfirst_person_character (+ (Variables|/Game/MyProject/Blueprints/Player/FirstPersonCharacter.FirstPersonCharacter_C|GetCurrentHealth _asfirst_person_character) 5e+01))))
      (Variables|/Game/MyProject/Blueprints/Player/FirstPersonCharacter.FirstPersonCharacter_C|SetPlayerGotTheFirstAid _asfirst_person_character true)
      (Class|NiagaraComponent|SetRenderingEnabled (Variables|Default|GetNS_Healing_1) false)
      (Variables|/Game/MyProject/Blueprints/Player/FirstPersonCharacter.FirstPersonCharacter_C|SetReloadingFirstAidKit _asfirst_person_character false)
      (Utilities|FlowControl|Delay 0.2)
      (Actor|DestroyActor))))

(fn ConstructionScript)
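; Rotating blade obstacle that damages the player's FirstPersonCharacter on contact.
; Tick passes through a short Delay, then adds a local rotation to the root, derived from the headset's base rotation X vector plus a fixed Y offset.
; An actor overlap with player character 0 subtracts a fixed amount directly from its CurrentHealth, with no clamp or death check here.
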(event EventBeginPlay)

(event Collision|EventActorBeginOverlap
  (params (OtherActor :type Actor%20Object%20Reference))
  (bind _returnvalue (Game|GetPlayerCharacter 0))
  ;[1 1 1] Remove Health points
  (if (== OtherActor _returnvalue)
    (bind _asfirst_person_character (Utilities|Casting|CastToFirstPersonCharacter _returnvalue))
    (Variables|/Game/MyProject/Blueprints/Player/FirstPersonCharacter.FirstPersonCharacter_C|SetCurrentHealth _asfirst_person_character (- (Variables|/Game/MyProject/Blueprints/Player/FirstPersonCharacter.FirstPersonCharacter_C|GetCurrentHealth _asfirst_person_character) 1e+01))))

(event EventTick
  (params (DeltaSeconds :type Float%20%28single-precision%29))
  ;[1 1 1] Rotate Object
  (Utilities|FlowControl|Delay 0.4)
  (Transformation|AddLocalRotation (Variables|Default|GetDefaultSceneRoot) (Math|Conversions|RotationFromXVector (+ (Math|Rotator|GetRotationXVector (.OutRotation (Class|OculusFunctionLibrary|GetBaseRotationandBaseOffsetinMeters))) "0.000000,1.000000, 0")) false false))

(fn ConstructionScript)
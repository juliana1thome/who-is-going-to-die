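; BP_ky_fireBall is a fire obstacle that damages the player while they stand inside its Box trigger.
; The Box's begin and end overlap events set and clear an IsInFire flag for the player character only.
; Tick runs through a short Delay, throttling it to periodic pulses that directly subtract a fixed amount from the FirstPersonCharacter's CurrentHealth while the flag is set.
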(event OnComponentBeginOverlap(Box)
  (params (OverlappedComponent :type Primitive%20Component%20Object%20Reference) (OtherActor :type Actor%20Object%20Reference) (OtherComp :type Primitive%20Component%20Object%20Reference) (OtherBodyIndex :type Integer) (bFromSweep :type Boolean) (SweepResult :type Hit%20Result%20Structure%20%28by%20ref%29))
  ;[1 1 1] When player gets on fire
  (if (== OtherActor (Game|GetPlayerCharacter 0))
    (Variables|Default|SetIsInFire true)))

(event OnComponentEndOverlap(Box)
  (params (OverlappedComponent :type Primitive%20Component%20Object%20Reference) (OtherActor :type Actor%20Object%20Reference) (OtherComp :type Primitive%20Component%20Object%20Reference) (OtherBodyIndex :type Integer))
  ;[1 1 1] When player gets off fire
  (if (== OtherActor (Game|GetPlayerCharacter 0))
    (Variables|Default|SetIsInFire false)))

(event EventTick
  (params (DeltaSeconds :type Float%20%28single-precision%29))
  ;[1 1 1] Check if player is on fire, if yes reduce its life, until it is dead
  (Utilities|FlowControl|Delay 0.25)
  (if (Variables|Default|GetIsInFire)
    (bind _asfirst_person_character (Utilities|Casting|CastToFirstPersonCharacter (Game|GetPlayerCharacter 0)))
    (Variables|/Game/MyProject/Blueprints/Player/FirstPersonCharacter.FirstPersonCharacter_C|SetCurrentHealth _asfirst_person_character (- (Variables|/Game/MyProject/Blueprints/Player/FirstPersonCharacter.FirstPersonCharacter_C|GetCurrentHealth _asfirst_person_character) 5.0))))

(fn ConstructionScript)
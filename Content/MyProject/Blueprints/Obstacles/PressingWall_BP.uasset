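; PressingWall_BP is an obstacle wall that moves back and forth and damages the player on contact.
; Tick applies one of two local transform offsets (HowMuch or HowMuchLess) every frame without sweep, chosen by ChangeDirection.
; A Delay in the Tick chain flips that flag about every five seconds, reversing the motion.
; Overlapping the player character subtracts a fixed amount from FirstPersonCharacter's CurrentHealth.
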(event EventBeginPlay)

(event Collision|EventActorBeginOverlap
  (params (OtherActor :type Actor%20Object%20Reference))
  (bind _returnvalue (Game|GetPlayerCharacter 0))
  ;[1 1 1] Remove Health points
  (if (== OtherActor _returnvalue)
    (bind _asfirst_person_character (Utilities|Casting|CastToFirstPersonCharacter _returnvalue))
    (Variables|/Game/MyProject/Blueprints/Player/FirstPersonCharacter.FirstPersonCharacter_C|SetCurrentHealth _asfirst_person_character (- (Variables|/Game/MyProject/Blueprints/Player/FirstPersonCharacter.FirstPersonCharacter_C|GetCurrentHealth _asfirst_person_character) 1e+01))))

(event EventTick
  (params (DeltaSeconds :type Float%20%28single-precision%29))
  ;[1 1 1] Make Wall go forward and comeback
  (if (Variables|Default|GetChangeDirection)
    (Class|Actor|AddActorLocalTransform (Math|Conversions|ToTransform(Vector) (Variables|Default|GetHowMuchLess?)) false false)
    (Utilities|FlowControl|Delay 5.0)
    (Variables|Default|SetChangeDirection false)
    (else
      (Class|Actor|AddActorLocalTransform (Math|Conversions|ToTransform(Vector) (Variables|Default|GetHowMuch?)) false false)
      (Utilities|FlowControl|Delay 5.0)
      (Variables|Default|SetChangeDirection true))))

(fn ConstructionScript)
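; Enemy AI character for the second objective that fires a laser at the player and dies when shot.
; After the first objective is acquired, a delayed Tick fires a forward line trace roughly every two seconds, with a random chance to damage the player on hit.
; Menu and player-state flags pause shooting.
; Projectile hits trigger a flag-guarded death that ragdolls the mesh, updates the player's kill count, then destroys the actor.
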(event OnComponentHit(Mesh)
  (params (HitComponent :type Primitive%20Component%20Object%20Reference) (OtherActor :type Actor%20Object%20Reference) (OtherComp :type Primitive%20Component%20Object%20Reference) (NormalImpulse :type Vector :default "0, 0, 0") (Hit :type Hit%20Result%20Structure%20%28by%20ref%29))
  ;[1 1 1] When Enemy Gets Shot
  (bind _asfirst_person_projectile (Utilities|Casting|CastToFirstPersonProjectile OtherActor))
  (if (== _asfirst_person_projectile OtherActor)
    (if (Variables|Default|GetAiIsDead)
      (CallFunction|Death)
      (Variables|Default|SetAiIsDead false)
      (Physics|AddImpulseatLocation (Variables|Character|GetMesh) (* (Transformation|GetVelocity OtherActor) 1e+01) "0, 0, 0" (.hitbonename Hit)))))

(event Custom|Death
  ;[1 1 1] Death
  (bind _asfirst_person_character (Utilities|Casting|CastToFirstPersonCharacter (Game|GetPlayerCharacter 0)))
  (bind _result (Math|Integer|IncrementInt (Variables|/Game/MyProject/Blueprints/Player/FirstPersonCharacter.FirstPersonCharacter_C|GetCurrentAIDeathTimes _asfirst_person_character))
    (:%20%20
      (Variables|/Game/MyProject/Blueprints/Player/FirstPersonCharacter.FirstPersonCharacter_C|SetCurrentAIDeathTimes _asfirst_person_character _result)
      (Collision|SetCollisionEnabled (Variables|Collision|GetCapsuleComponent) "NoCollision")
      (Physics|SetSimulatePhysics (Variables|Character|GetMesh) true)
      (Variables|Default|SetAiIsDead true)
      (Utilities|FlowControl|Delay 1.0)
      (Actor|DestroyActor)
      (Default|AIDeath _asfirst_person_character))))

(event EventTick
  (params (DeltaSeconds :type Float%20%28single-precision%29))
  (bind _returnvalue (Game|GetPlayerCharacter 0))
  (bind _capsulecomponent (Variables|Collision|GetCapsuleComponent))
  (bind _returnvalue_2 (Transformation|GetWorldLocation _capsulecomponent))
  ;[1 1 1] Shoot with Laser (Line Trace)
  (Utilities|FlowControl|Delay 2.0)
  (bind _asfirst_person_character (Utilities|Casting|CastToFirstPersonCharacter (Game|GetPlayerCharacter 0)))
  (if (Variables|/Game/MyProject/Blueprints/Player/FirstPersonCharacter.FirstPersonCharacter_C|GetIsFirstObjectAquired _asfirst_person_character)
    (Variables|Default|SetEnemyHitOrNot (Math|Random|RandomBool)) ; Making enemy hit the player randomly, like it make mistakes
    (if (not (Variables|/Game/MyProject/Blueprints/Player/FirstPersonCharacter.FirstPersonCharacter_C|GetInstructionsMenuOpen _asfirst_person_character))
      (if (Variables|/Game/MyProject/Blueprints/Player/FirstPersonCharacter.FirstPersonCharacter_C|GetEnemyCanContinueShooting _asfirst_person_character) ; Check if it is dead, if yes it can move, so when the player restart, it does not know where the enemy is. However, the enemy cannot shoot while player is dead
        (bind _asfirst_person_character_2 (Utilities|Casting|CastToFirstPersonCharacter (Game|GetPlayerCharacter 0)))
        (if (not (Variables|/Game/MyProject/Blueprints/Player/FirstPersonCharacter.FirstPersonCharacter_C|GetInstructionsMenuOpen _asfirst_person_character_2))
          (bind _outhit (Collision|LineTraceByChannel (+ _returnvalue_2 "0,-5.000000,90.000000") (+ _returnvalue_2 (* (Math|Vector|GetForwardVector (Transformation|GetWorldRotation _capsulecomponent)) 1.3e+03)) "TraceTypeQuery2" false 0 "ForDuration" true "(R=0.640625,G=0.000000,B=0.000000,A=1.000000)" "(R=0.447917,G=0.000000,B=0.007311,A=1.000000)" 1.0))
          (Audio|PlaySoundatLocation "/Game/FirstPerson/Audio/FirstPersonTemplateWeaponFire02.FirstPersonTemplateWeaponFire02" (Transformation|GetWorldLocation (Variables|Default|GetFP_Gun)) "0, 0, 0" 0.1 1.0 0.0 0 0 0) ; Play firing sound
          (if (== _returnvalue (.HitActor (Collision|BreakHitResult _outhit)))
            (if (Variables|Default|GetEnemyHitOrNot)
              (bind _asfirst_person_character_3 (Utilities|Casting|CastToFirstPersonCharacter _returnvalue))
              (Variables|/Game/MyProject/Blueprints/Player/FirstPersonCharacter.FirstPersonCharacter_C|SetCurrentHealth _asfirst_person_character_3 (- (Variables|/Game/MyProject/Blueprints/Player/FirstPersonCharacter.FirstPersonCharacter_C|GetCurrentHealth _asfirst_person_character_3) 3e+01)))))))))

(fn ConstructionScript)